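; BP_DeckPlayerState is a player state that holds the player's Soul Shards currency for Dead Man's Deck.
; AddSoulShards increases the balance for positive amounts only, and SpendSoulShards deducts only when the amount is positive and affordable, returning whether it succeeded.
; Both broadcast OnSoulShardsChanged with the new total, and GetSoulShards exposes the current balance.
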(event EventBeginPlay)

(event EventTick
  (params (DeltaSeconds :type Float%20%28single-precision%29)))

(fn ConstructionScript)

(fn AddSoulShards
  (params (Amount :type Integer))
  (if (> Amount (Class|KismetSystemLibrary|MakeLiteralInteger))
    (Variables|Souls|SetSoulShards (+ (Variables|Souls|GetSoulShards) Amount))
    (Default|CallOnSoulShardsChanged (Variables|Souls|GetSoulShards))))

(fn SpendSoulShards
  (params (Amount :type Integer))
  (if (and (> Amount (Class|KismetSystemLibrary|MakeLiteralInteger)) (>= (Variables|Souls|GetSoulShards) Amount))
    (Variables|Souls|SetSoulShards (- (Variables|Souls|GetSoulShards) Amount))
    (Default|CallOnSoulShardsChanged (Variables|Souls|GetSoulShards))
    (return true)
    (else
      (return false))))

(fn GetSoulShards
  (return (Variables|Souls|GetSoulShards)))