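; Health component for Dead Man's Deck that tracks an owning actor's health and death state.
; On BeginPlay it fills health to max and binds to the owner's TakeAnyDamage, routing damage into ApplyHealthDamage.
; That clamps health, broadcasts OnDamaged, and at zero sets IsDead once and broadcasts OnDeath.
; Heal restores health only while alive, and GetHealthPercent returns health on a 0–100 scale.
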(event Custom|OnTakeAnyDamage_Event
  (params (DamagedActor :type Actor%20Object%20Reference) (Damage :type Float%20%28single-precision%29) (DamageType :type Damage%20Type%20Object%20Reference) (InstigatedBy :type Controller%20Object%20Reference) (DamageCauser :type Actor%20Object%20Reference))
  (CallFunction|ApplyHealthDamage Damage))

(event Custom|OnTakeAnyDamage_Event_0
  (params (DamagedActor :type Actor%20Object%20Reference) (Damage :type Float%20%28single-precision%29) (DamageType :type Damage%20Type%20Object%20Reference) (InstigatedBy :type Controller%20Object%20Reference) (DamageCauser :type Actor%20Object%20Reference)))

(event EventBeginPlay
  (Variables|Health|SetCurrentHealth (Variables|Health|GetMaxHealth))
  (Variables|Health|SetbIsDead false)
  (EventDispatchers|AssignOnTakeAnyDamage (Components|GetOwner) (delegate Custom|OnTakeAnyDamage_Event)))

(event EventTick
  (params (DeltaSeconds :type Float%20%28single-precision%29)))

(fn ApplyHealthDamage
  (params (Amount :type Float%20%28double-precision%29))
  (if (and (> Amount (Math|Float|MakeLiteralFloat 0.0)) (not (Variables|Health|GetbIsDead)))
    (Variables|Health|SetCurrentHealth (Math|Float|Clamp(Float) (- (Variables|Health|GetCurrentHealth) Amount) 0.0 (Variables|Health|GetMaxHealth)))
    (Default|CallOnDamaged Amount (Variables|Health|GetCurrentHealth))
    (if (<= (Variables|Health|GetCurrentHealth) (Math|Float|MakeLiteralFloat 0.0))
      (Variables|Health|SetbIsDead true)
      (Default|CallOnDeath (Components|GetOwner)))))

(fn Heal
  (params (Amount :type Float%20%28double-precision%29))
  (if (and (> Amount (Math|Float|MakeLiteralFloat 0.0)) (not (Variables|Health|GetbIsDead)))
    (Variables|Health|SetCurrentHealth (Math|Float|Clamp(Float) (+ (Variables|Health|GetCurrentHealth) Amount) 0.0 (Variables|Health|GetMaxHealth)))))

(fn GetHealthPercent
  (return (* (Math|Float|SafeDivide (Variables|Health|GetCurrentHealth) (Variables|Health|GetMaxHealth)) (Math|Float|MakeLiteralFloat 1e+02))))