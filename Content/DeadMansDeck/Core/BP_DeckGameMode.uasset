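; Game mode for Dead Man's Deck that runs enemy waves of skeleton rafts from the DT_Waves data table.
; Each wave row sets raft count, skeletons per raft and spawn interval; a looping timer spawns rafts alternately on random starboard and port lanes collected at BeginPlay.
; Enemies register and unregister to keep an alive count.
; A wave ends when none remain to spawn or fight, then the next starts after a short delay.
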(event EventBeginPlay
  (CallFunction|CollectLanes)
  (bind _outrownames (DataTable|GetDataTableRowNames "/Game/DeadMansDeck/Waves/DT_Waves.DT_Waves"))
  (Variables|Waves|SetWaveRowNames _outrownames)
  (if (Variables|Waves|GetbAutoStart)
    (Utilities|Time|SetTimerbyFunctionName self "StartNextWave" (Variables|Waves|GetFirstWaveDelay))))

(fn ConstructionScript)

(fn StartNextWave
  (Variables|Waves|SetCurrentWave (+ (Variables|Waves|GetCurrentWave) (Class|KismetSystemLibrary|MakeLiteralInteger 1)))
  (bind _returnvalue (Utilities|GetDataTableRow "/Game/DeadMansDeck/Waves/DT_Waves.DT_Waves" (Utilities|Array|Get(acopy) (Variables|Waves|GetWaveRowNames) (- (Variables|Waves|GetCurrentWave) (Class|KismetSystemLibrary|MakeLiteralInteger 1))))
    (:then
      (Variables|Waves|SetRaftsToSpawn (* (.RaftsPerSide (Utilities|Struct|BreakS_WaveData _returnvalue)) (Class|KismetSystemLibrary|MakeLiteralInteger 2)))
      (Variables|Waves|SetWaveSkeletonsPerRaft (.SkeletonsPerRaft (Utilities|Struct|BreakS_WaveData _returnvalue)))
      (Variables|Waves|SetbWaveActive true)
      (Default|CallOnWaveStarted (Variables|Waves|GetCurrentWave))
      (Development|PrintString (Utilities|String|Append "Wave " (Utilities|String|ToString(Integer) (Variables|Waves|GetCurrentWave))) true true "(R=0.000000,G=0.660000,B=1.000000,A=1.000000)" 4.0)
      (CallFunction|SpawnNextRaft)
      (Utilities|Time|SetTimerbyFunctionName self "SpawnNextRaft" (.SpawnInterval (Utilities|Struct|BreakS_WaveData _returnvalue)) true))))

(fn SpawnNextRaft
  (if (<= (Variables|Waves|GetRaftsToSpawn) (Class|KismetSystemLibrary|MakeLiteralInteger))
    (Utilities|Time|ClearTimerbyFunctionName self "SpawnNextRaft")
    (else
      (LocalVariables|SetPickedLane (select (Variables|Waves|GetbSpawnStarboard) (Utilities|Array|Get(acopy) (Variables|Waves|GetStarboardLanes) (Math|Random|RandomIntegerinRange 0 (- (Utilities|Array|Length (Variables|Waves|GetStarboardLanes)) (Class|KismetSystemLibrary|MakeLiteralInteger 1)))) (Utilities|Array|Get(acopy) (Variables|Waves|GetPortLanes) (Math|Random|RandomIntegerinRange 0 (- (Utilities|Array|Length (Variables|Waves|GetPortLanes)) (Class|KismetSystemLibrary|MakeLiteralInteger 1))))))
      (Variables|Waves|SetbSpawnStarboard (not (Variables|Waves|GetbSpawnStarboard)))
      (Variables|Waves|SetRaftsToSpawn (- (Variables|Waves|GetRaftsToSpawn) (Class|KismetSystemLibrary|MakeLiteralInteger 1)))
      (Utilities|IsValid (LocalVariables|GetPickedLane)
        (:Is%20Valid
          (bind _raft (Default|SpawnRaft (LocalVariables|GetPickedLane) (Variables|/Game/DeadMansDeck/Rafts/BP_RaftLane.BP_RaftLane_C|GetRaftSpeed (LocalVariables|GetPickedLane))))
          (Variables|/Game/DeadMansDeck/Rafts/BP_Raft.BP_Raft_C|SetSkeletonCount _raft (Variables|Waves|GetWaveSkeletonsPerRaft)))))))

(fn RegisterEnemy
  (Variables|Waves|SetAliveEnemies (+ (Variables|Waves|GetAliveEnemies) (Class|KismetSystemLibrary|MakeLiteralInteger 1))))

(fn UnregisterEnemy
  (Variables|Waves|SetAliveEnemies (Math|Integer|Max(Integer) (- (Variables|Waves|GetAliveEnemies) (Class|KismetSystemLibrary|MakeLiteralInteger 1))))
  (CallFunction|CheckWaveEnd))

(fn CheckWaveEnd
  (if (and (Variables|Waves|GetbWaveActive) (and (<= (Variables|Waves|GetRaftsToSpawn) (Class|KismetSystemLibrary|MakeLiteralInteger)) (<= (Variables|Waves|GetAliveEnemies) (Class|KismetSystemLibrary|MakeLiteralInteger))))
    (CallFunction|EndWave)))

(fn EndWave
  (Variables|Waves|SetbWaveActive false)
  (Default|CallOnWaveEnded (Variables|Waves|GetCurrentWave))
  (Development|PrintString (Utilities|String|Append (Utilities|String|Append "Wave " (Utilities|String|ToString(Integer) (Variables|Waves|GetCurrentWave))) " cleared") true true "(R=0.000000,G=0.660000,B=1.000000,A=1.000000)" 4.0)
  (if (< (Variables|Waves|GetCurrentWave) (Utilities|Array|Length (Variables|Waves|GetWaveRowNames)))
    (Utilities|Time|SetTimerbyFunctionName self "StartNextWave" 3.0)))

(fn CollectLanes
  (bind _outactors (Actor|GetAllActorsOfClass "/Game/DeadMansDeck/Rafts/BP_RaftLane.BP_RaftLane_C"))
  (for _array_element _outactors
    (if (Variables|/Game/DeadMansDeck/Rafts/BP_RaftLane.BP_RaftLane_C|GetbStarboard _array_element)
      (Utilities|Array|Add (Variables|Waves|GetStarboardLanes) _array_element)
      (else
        (Utilities|Array|Add (Variables|Waves|GetPortLanes) _array_element)))))