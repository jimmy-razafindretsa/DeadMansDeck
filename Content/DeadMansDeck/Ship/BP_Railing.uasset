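; Ship railing actor that switches between intact and broken states.
; Break and Repair act only on an actual state change, then refresh the visuals and broadcast OnRailingStateChanged with the railing and its new state.
; ApplyVisualState, also run at construction, shows the mesh matching IsBroken and disables the intact mesh's collision while broken.
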(event EventBeginPlay)

(event Collision|EventActorBeginOverlap
  (params (OtherActor :type Actor%20Object%20Reference)))

(event EventTick
  (params (DeltaSeconds :type Float%20%28single-precision%29)))

(fn ConstructionScript
  (CallFunction|ApplyVisualState))

(fn Break
  (if (not (Variables|Railing|GetbIsBroken))
    (Variables|Railing|SetbIsBroken true)
    (CallFunction|ApplyVisualState)
    (Default|CallOnRailingStateChanged self true)))

(fn Repair
  (if (Variables|Railing|GetbIsBroken)
    (Variables|Railing|SetbIsBroken false)
    (CallFunction|ApplyVisualState)
    (Default|CallOnRailingStateChanged self false)))

(fn ApplyVisualState
  (bind _bisbroken (Variables|Railing|GetbIsBroken))
  (bind _intactmesh (Variables|Default|GetIntactMesh))
  (Rendering|SetVisibility _intactmesh (not _bisbroken) false)
  (Rendering|SetVisibility (Variables|Default|GetBrokenMesh) _bisbroken false)
  (if _bisbroken
    (Collision|SetCollisionEnabled _intactmesh "NoCollision")
    (else
      (Collision|SetCollisionEnabled _intactmesh "QueryAndPhysics"))))