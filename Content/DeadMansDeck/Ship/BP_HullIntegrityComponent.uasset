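; Actor component that tracks a ship's hull integrity, starting at maximum on BeginPlay.
; Damage and repair functions ignore negative amounts and route through SetHull, which clamps the value between zero and the maximum.
; SetHull broadcasts OnHullChanged with the delta only on real changes, and OnHullDestroyed when the hull drops to zero from above.
; GetHullPercent exposes the current hull as a safely divided percentage.
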(event EventBeginPlay
  (bind _maxhull (Variables|Hull|GetMaxHull))
  (Variables|Hull|SetCurrentHull _maxhull)
  (Default|CallOnHullChanged _maxhull 0.0))

(event EventTick
  (params (DeltaSeconds :type Float%20%28single-precision%29)))

(fn SetHull
  (params (NewValue :type Float%20%28double-precision%29))
  (LocalVariables|SetOldHull (Variables|Hull|GetCurrentHull))
  (LocalVariables|SetNewHull (Math|Float|Clamp(Float) NewValue 0.0 (Variables|Hull|GetMaxHull)))
  (if (not (Math|Float|NearlyEqual(Float) (LocalVariables|GetNewHull) (LocalVariables|GetOldHull) 1e-06))
    (Variables|Hull|SetCurrentHull (LocalVariables|GetNewHull))
    (Default|CallOnHullChanged (LocalVariables|GetNewHull) (- (LocalVariables|GetNewHull) (LocalVariables|GetOldHull)))
    (if (and (<= (LocalVariables|GetNewHull) (Math|Float|MakeLiteralFloat 0.0)) (> (LocalVariables|GetOldHull) (Math|Float|MakeLiteralFloat 0.0)))
      (Default|CallOnHullDestroyed))))

(fn ApplyHullDamage
  (params (Amount :type Float%20%28double-precision%29))
  (CallFunction|SetHull (- (Variables|Hull|GetCurrentHull) (Math|Float|Max(Float) Amount 0.0))))

(fn RepairHull
  (params (Amount :type Float%20%28double-precision%29))
  (CallFunction|SetHull (+ (Variables|Hull|GetCurrentHull) (Math|Float|Max(Float) Amount 0.0))))

(fn GetHullPercent
  (return (* (Math|Float|SafeDivide (Variables|Hull|GetCurrentHull) (Variables|Hull|GetMaxHull)) (Math|Float|MakeLiteralFloat 1e+02))))