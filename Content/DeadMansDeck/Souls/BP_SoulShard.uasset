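; BP_SoulShard is a pickup that grants soul shards when the captain overlaps it.
; Collect runs once, adds its Value to player 0's BP_DeckPlayerState, then destroys the actor, which also happens if the cast fails.
; The construction script makes the Pickup component overlap all dynamic objects and turns off collision on the Orb.
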(event EventBeginPlay)

(event Collision|EventActorBeginOverlap
  (params (OtherActor :type Actor%20Object%20Reference))
  (Utilities|Casting|CastToBP_Captain OtherActor)
  (CallFunction|Collect))

(event EventTick
  (params (DeltaSeconds :type Float%20%28single-precision%29)))

(fn ConstructionScript
  (Collision|SetCollisionProfileName (Variables|Default|GetPickup) "OverlapAllDynamic" true :!class /Script/Engine.PrimitiveComponent)
  (Collision|SetCollisionEnabled (Variables|Default|GetOrb) "NoCollision"))

(fn Collect
  (if (not (Variables|Souls|GetbCollected))
    (Variables|Souls|SetbCollected true)
    (bind _asbp_deck_player_state (Utilities|Casting|CastToBP_DeckPlayerState (Game|GetPlayerState 0))
      (:then
        (Default|AddSoulShards _asbp_deck_player_state (Variables|Souls|GetValue))
        (Actor|DestroyActor))
      (:CastFailed
        (Actor|DestroyActor)))))