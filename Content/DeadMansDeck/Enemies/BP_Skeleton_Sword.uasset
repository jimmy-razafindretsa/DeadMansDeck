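; Sword skeleton enemy Blueprint that handles its own death.
; On BeginPlay it binds to the Health component's OnDeath, which calls Die.
; Die detaches the controller, disables movement and capsule collision, and switches the mesh to physics ragdoll.
; It then broadcasts OnSkeletonDied with itself and sets a short lifespan so the corpse is removed.
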(event Custom|OnDeath_Event
  (params (DeadActor :type Actor%20Object%20Reference))
  (CallFunction|Die))

(event Custom|OnDeath_Event_0
  (params (DeadActor :type Actor%20Object%20Reference)))

(event EventBeginPlay
  (EventDispatchers|AssignOnDeath (Variables|Default|GetHealth) (delegate Custom|OnDeath_Event)))

(event Collision|EventActorBeginOverlap
  (params (OtherActor :type Actor%20Object%20Reference)))

(event EventTick
  (params (DeltaSeconds :type Float%20%28single-precision%29)))

(fn ConstructionScript)

(fn Die
  (bind _mesh (Variables|Character|GetMesh))
  (Class|Pawn|DetachfromControllerPendingDestroy)
  (Pawn|Components|CharacterMovement|DisableMovement (Variables|Character|GetCharacterMovement))
  (Collision|SetCollisionEnabled (Variables|Collision|GetCapsuleComponent) "NoCollision")
  (Collision|SetCollisionProfileName _mesh "Ragdoll" true :!class /Script/Engine.PrimitiveComponent)
  (Physics|SetSimulatePhysics _mesh true)
  (Default|CallOnSkeletonDied self)
  (Actor|SetLifeSpan 6.0))