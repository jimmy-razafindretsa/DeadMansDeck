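; BP_Cannon is a possessable cannon that the player can man through interaction, offering a "Man the cannon" prompt.
; Interact stores the instigator as MountedCaptain, hides it and possesses the cannon, provided nobody is already mounted.
; On possession it swaps the default and deck Enhanced Input contexts for the artillery one.
; IA_Interact triggers Dismount, which restores those contexts, unhides and repossesses the captain, then clears the reference.
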(event Input|EnhancedActionEvents|EnhancedInputActionIA_Interact
  (params (ActionValue :type Boolean) (ElapsedSeconds :type Float%20%28double-precision%29) (TriggeredSeconds :type Float%20%28double-precision%29) (InputAction :type Input%20Action%20Object%20Reference :default "/Game/DeadMansDeck/Input/Actions/IA_Interact.IA_Interact"))
  (:Started
    (CallFunction|Dismount)))

(event EventBeginPlay)

(event Collision|EventActorBeginOverlap
  (params (OtherActor :type Actor%20Object%20Reference)))

(event EventTick
  (params (DeltaSeconds :type Float%20%28single-precision%29)))

(event EventInteract
  (params (Instigator :type Pawn%20Object%20Reference))
  (Utilities|IsValid (Variables|Default|GetMountedCaptain)
    (:Is%20Not%20Valid
      (bind _asplayer_controller (Utilities|Casting|CastToPlayerController (Pawn|GetController Instigator)))
      (Variables|Default|SetMountedCaptain Instigator)
      (Rendering|SetActorHiddenInGame Instigator true)
      (Pawn|Possess _asplayer_controller self))))

(event EventPossessed
  (params (NewController :type Controller%20Object%20Reference))
  (bind _asplayer_controller (Utilities|Casting|CastToPlayerController NewController))
  (Input|RemoveMappingContext (PlayerController|LocalPlayerSubsystems|GetEnhancedInputLocalPlayerSubsystem _asplayer_controller) "/Game/Input/IMC_Default.IMC_Default" "(bIgnoreAllPressedKeysUntilRelease=True,bForceImmediately=False,bNotifyUserSettings=False)")
  (Input|RemoveMappingContext (PlayerController|LocalPlayerSubsystems|GetEnhancedInputLocalPlayerSubsystem _asplayer_controller) "/Game/DeadMansDeck/Input/IMC_Deck.IMC_Deck" "(bIgnoreAllPressedKeysUntilRelease=True,bForceImmediately=False,bNotifyUserSettings=False)")
  (Input|AddMappingContext (PlayerController|LocalPlayerSubsystems|GetEnhancedInputLocalPlayerSubsystem _asplayer_controller) "/Game/DeadMansDeck/Input/IMC_Artillery.IMC_Artillery" 0 "(bIgnoreAllPressedKeysUntilRelease=True,bForceImmediately=False,bNotifyUserSettings=False)"))

(fn ConstructionScript)

(fn Dismount
  (bind _asplayer_controller (Utilities|Casting|CastToPlayerController (Pawn|GetController self)))
  (Input|RemoveMappingContext (PlayerController|LocalPlayerSubsystems|GetEnhancedInputLocalPlayerSubsystem _asplayer_controller) "/Game/DeadMansDeck/Input/IMC_Artillery.IMC_Artillery" "(bIgnoreAllPressedKeysUntilRelease=True,bForceImmediately=False,bNotifyUserSettings=False)")
  (Input|AddMappingContext (PlayerController|LocalPlayerSubsystems|GetEnhancedInputLocalPlayerSubsystem _asplayer_controller) "/Game/Input/IMC_Default.IMC_Default" 0 "(bIgnoreAllPressedKeysUntilRelease=True,bForceImmediately=False,bNotifyUserSettings=False)")
  (Input|AddMappingContext (PlayerController|LocalPlayerSubsystems|GetEnhancedInputLocalPlayerSubsystem _asplayer_controller) "/Game/DeadMansDeck/Input/IMC_Deck.IMC_Deck" 0 "(bIgnoreAllPressedKeysUntilRelease=True,bForceImmediately=False,bNotifyUserSettings=False)")
  (Rendering|SetActorHiddenInGame (Variables|Default|GetMountedCaptain) false)
  (Pawn|Possess _asplayer_controller (Variables|Default|GetMountedCaptain))
  (Variables|Default|SetMountedCaptain 0))

(fn GetPrompt
  (return (Utilities|Text|MakeLiteralText "Man the cannon")))