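; BP_Cannonball is a cannonball actor that deals direct and area damage when it hits something.
; On BeginPlay its Collision component ignores the instigator while moving, so the ball does not collide with whoever fired it.
; On Hit it damages the struck actor, applies radial damage around the impact point, both credited to the instigator's controller, then destroys itself.
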(event EventBeginPlay
  (Collision|IgnoreActorwhenMoving (Variables|Default|GetCollision) (Game|GetInstigator) true))

(event Collision|EventActorBeginOverlap
  (params (OtherActor :type Actor%20Object%20Reference)))

(event EventTick
  (params (DeltaSeconds :type Float%20%28single-precision%29)))

(event Collision|EventHit
  (params (MyComp :type Primitive%20Component%20Object%20Reference) (Other :type Actor%20Object%20Reference) (OtherComp :type Primitive%20Component%20Object%20Reference) (bSelfMoved :type Boolean) (HitLocation :type Vector :default "0, 0, 0") (HitNormal :type Vector :default "0, 0, 0") (NormalImpulse :type Vector :default "0, 0, 0") (Hit :type Hit%20Result%20Structure%20%28by%20ref%29))
  (bind _returnvalue (Game|GetInstigatorController))
  (bind _self self)
  (Game|Damage|ApplyDamage Other (Variables|Cannonball|GetDamage) _returnvalue _self)
  (Game|Damage|ApplyRadialDamage (Variables|Cannonball|GetRadialDamage) HitLocation (Variables|Cannonball|GetDamageRadius) 0 0 _self _returnvalue false "ECC_Visibility")
  (Actor|DestroyActor _self))

(fn ConstructionScript)