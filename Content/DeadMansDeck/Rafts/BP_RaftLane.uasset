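; BP_RaftLane is an actor that defines a curved spline lane, apparently for rafts in Dead Man's Deck.
; The construction script rebuilds three local spline points from SeaDistance and Sway, running from the far sea end through an opposite-swayed midpoint to the actor origin.
; GetLaneLength exposes the spline length, and the actor has no active event logic.
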(event EventBeginPlay)

(event Collision|EventActorBeginOverlap
  (params (OtherActor :type Actor%20Object%20Reference)))

(event EventTick
  (params (DeltaSeconds :type Float%20%28single-precision%29)))

(fn ConstructionScript
  (bind _spline (Variables|Default|GetSpline))
  (bind _seadistance (Variables|Lane|GetSeaDistance))
  (bind _sway (Variables|Lane|GetSway))
  (Spline|ClearSplinePoints _spline false)
  (Spline|AddSplinePoint _spline (Math|Vector|MakeVector _seadistance _sway 0.0) "Local" false)
  (Spline|AddSplinePoint _spline (Math|Vector|MakeVector (* _seadistance (Math|Float|MakeLiteralFloat 0.5)) (* _sway (Math|Float|MakeLiteralFloat -0.5)) 0.0) "Local" false)
  (Spline|AddSplinePoint _spline (Math|Vector|MakeVector 0.0 0.0 0.0) "Local" true))

(fn GetLaneLength
  (return (Spline|GetSplineLength (Variables|Default|GetSpline))))