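; Enemy raft that rides a lane spline toward the ship and registers with the deck game mode as an enemy.
; On reaching the lane's end it damages the hull by a percentage of max, breaks the nearest railing and spawns a row of skeleton boarders.
; A single hit above the damage threshold shatters it into physics-launched planks with an explosion.
; Either outcome unregisters it through a once-only guard.
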(event EventBeginPlay
  (bind _lane (Variables|Raft|GetLane))
  (Utilities|IsValid _lane
    (:Is%20Valid
      (CallFunction|InitRaft _lane (Variables|Raft|GetSpeed)))))

(event Collision|EventActorBeginOverlap
  (params (OtherActor :type Actor%20Object%20Reference)))

(event EventTick
  (params (DeltaSeconds :type Float%20%28single-precision%29))
  (bind _lane (Variables|Raft|GetLane))
  (Utilities|IsValid _lane
    (:Is%20Valid
      (if (not (Variables|Raft|GetbReachedHull))
        (bind _length (Default|GetLaneLength _lane))
        (Variables|Raft|SetDistanceOnLane (Math|Float|Min(Float) (+ (Variables|Raft|GetDistanceOnLane) (* (Variables|Raft|GetSpeed) DeltaSeconds)) _length))
        (CallFunction|MovetoDistance (Math|Float|Min(Float) (+ (Variables|Raft|GetDistanceOnLane) (* (Variables|Raft|GetSpeed) DeltaSeconds)) _length))
        (if (>= (Math|Float|Min(Float) (+ (Variables|Raft|GetDistanceOnLane) (* (Variables|Raft|GetSpeed) DeltaSeconds)) _length) _length)
          (Variables|Raft|SetbReachedHull true)
          (Actor|Tick|SetActorTickEnabled false)
          (CallFunction|ImpactHull)
          (Default|CallOnReachedHull self))))))

(event Game|Damage|EventAnyDamage
  (params (Damage :type Float%20%28single-precision%29) (DamageType :type Damage%20Type%20Object%20Reference) (InstigatedBy :type Controller%20Object%20Reference) (DamageCauser :type Actor%20Object%20Reference))
  (if (>= Damage (Variables|Raft|GetDamageToBreak))
    (CallFunction|BreakApart)))

(fn ConstructionScript
  (Collision|SetCollisionEnabled (Variables|Default|GetPlank1) "NoCollision")
  (Collision|SetCollisionEnabled (Variables|Default|GetPlank2) "NoCollision")
  (Collision|SetCollisionEnabled (Variables|Default|GetPlank3) "NoCollision")
  (Collision|SetCollisionEnabled (Variables|Default|GetPlank4) "NoCollision"))

(fn InitRaft
  (params (InLane :type BP%20Raft%20Lane%20Object%20Reference) (InSpeed :type Float%20%28double-precision%29))
  (Variables|Raft|SetLane InLane)
  (Variables|Raft|SetSpeed InSpeed)
  (Variables|Raft|SetDistanceOnLane 0.0)
  (Variables|Raft|SetbReachedHull false)
  (Actor|Tick|SetActorTickEnabled true)
  (CallFunction|MovetoDistance 0.0)
  (CallFunction|RegisterwithGameMode))

(fn MovetoDistance
  (params (Distance :type Float%20%28double-precision%29))
  (bind _lane (Variables|Raft|GetLane))
  (bind _spline (Variables|/Game/DeadMansDeck/Rafts/BP_RaftLane.BP_RaftLane_C|GetSpline _lane))
  (Transformation|SetActorLocationAndRotation (Spline|GetLocationatDistanceAlongSpline _spline Distance "World") (Spline|GetRotationatDistanceAlongSpline _spline Distance "World") false true))

(fn BreakApart
  (bind _raftmesh (Variables|Default|GetRaftMesh))
  (if (not (Variables|Raft|GetbDestroyed))
    (Variables|Raft|SetbDestroyed true)
    (Actor|Tick|SetActorTickEnabled false)
    (Rendering|SetVisibility _raftmesh false false)
    (Collision|SetCollisionEnabled _raftmesh "NoCollision")
    (CallFunction|LaunchPlank (Variables|Default|GetPlank1))
    (CallFunction|LaunchPlank (Variables|Default|GetPlank2))
    (CallFunction|LaunchPlank (Variables|Default|GetPlank3))
    (CallFunction|LaunchPlank (Variables|Default|GetPlank4))
    (Niagara|SpawnSystematLocation "/Niagara/DefaultAssets/Templates/Systems/SimpleExplosion.SimpleExplosion" (Transformation|GetActorLocation))
    (Default|CallOnRaftDestroyed self)
    (CallFunction|ResolveEnemy)
    (Actor|SetLifeSpan 6.0)))

(fn LaunchPlank
  (params (Plank :type Static%20Mesh%20Component%20Object%20Reference))
  (Rendering|SetVisibility Plank true false)
  (Collision|SetCollisionEnabled Plank "PhysicsOnly")
  (Physics|SetSimulatePhysics Plank true)
  (Physics|AddImpulse Plank (* (Math|Random|RandomUnitVectorinConeinDegrees (Math|Vector|MakeVector 0.0 0.0 1.0) 6e+01) (Math|Float|MakeLiteralFloat 6e+02)) "None" true))

(fn ImpactHull
  (CallFunction|DamageHull)
  (bind _railing (CallFunction|FindNearestRailing))
  (Utilities|IsValid _railing
    (:Is%20Valid
      (Default|Break _railing)
      (CallFunction|SpawnBoarders _railing)
      (CallFunction|ResolveEnemy))
    (:Is%20Not%20Valid
      (CallFunction|ResolveEnemy))))

(fn FindNearestRailing
  (LocalVariables|SetBestDistance 1e+09)
  (bind _outactors (Actor|GetAllActorsOfClass "/Game/DeadMansDeck/Ship/BP_Railing.BP_Railing_C"))
  (for _array_element _outactors
    (if (< (Transformation|GetDistanceTo self _array_element) (LocalVariables|GetBestDistance))
      (LocalVariables|SetBestDistance (Transformation|GetDistanceTo self _array_element))
      (LocalVariables|SetBestRailing _array_element)))
  (return (LocalVariables|GetBestRailing)))

(fn DamageHull
  (bind _asbp_deck_game_mode (Utilities|Casting|CastToBP_DeckGameMode (Game|GetGameMode)))
  (Default|ApplyHullDamage (Variables|/Game/DeadMansDeck/Core/BP_DeckGameMode.BP_DeckGameMode_C|GetHullIntegrity _asbp_deck_game_mode) (/ (* (Variables|/Game/DeadMansDeck/Ship/BP_HullIntegrityComponent.BP_HullIntegrityComponent_C|GetMaxHull (Variables|/Game/DeadMansDeck/Core/BP_DeckGameMode.BP_DeckGameMode_C|GetHullIntegrity _asbp_deck_game_mode)) (Variables|Raft|GetHullDamagePercent)) (Math|Float|MakeLiteralFloat 1e+02))))

(fn SpawnBoarders
  (params (Railing :type BP%20Railing%20Object%20Reference))
  (bind _returnvalue (Transformation|GetActorLocation))
  (bind _skeletoncount (Variables|Boarders|GetSkeletonCount))
  (for _index (range 0 (- _skeletoncount (Class|KismetSystemLibrary|MakeLiteralInteger 1)))
    (bind _returnvalue_2 (Game|SpawnActorfromClass "/Game/DeadMansDeck/Enemies/BP_Skeleton_Sword.BP_Skeleton_Sword_C" (Math|Transform|MakeTransform (Math|Vector|MakeVector (+ (.X (Math|Vector|BreakVector _returnvalue)) (* (- (Math|Conversions|ToFloat(Integer) _index) (/ (- (Math|Conversions|ToFloat(Integer) _skeletoncount) (Math|Float|MakeLiteralFloat 1.0)) (Math|Float|MakeLiteralFloat 2.0))) (Variables|Boarders|GetSkeletonSpacing))) (.Y (Math|Vector|BreakVector _returnvalue)) (+ (.Z (Math|Vector|BreakVector _returnvalue)) (Math|Float|MakeLiteralFloat 1e+02)))) "AlwaysSpawn" "MultiplyWithRoot" 0 0))
    (Default|BeginBoarding _returnvalue_2 Railing)))

(fn RegisterwithGameMode
  (bind _asbp_deck_game_mode (Utilities|Casting|CastToBP_DeckGameMode (Game|GetGameMode)))
  (Default|RegisterEnemy _asbp_deck_game_mode))

(fn ResolveEnemy
  (if (not (Variables|Raft|GetbResolved))
    (Variables|Raft|SetbResolved true)
    (bind _asbp_deck_game_mode (Utilities|Casting|CastToBP_DeckGameMode (Game|GetGameMode)))
    (Default|UnregisterEnemy _asbp_deck_game_mode)))